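; ATable_BP is a table actor in ingame level 01 that drops into place from above when play begins.
; On BeginPlay, a SkyDrop timeline lerps the Table component's relative location from high up down to its resting height.
; When that finishes, a Shake timeline adds a landing wobble, pitching the table and using the absolute curve value to bounce it slightly upward.
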(event `self.ReceiveBeginPlay`
  (bind _table (`self.Table`))
  (bind (_direction _fall) (`Timeline|Sky drop` :!via `PlayFromStart`)
    (:`Update`
      (`SceneComponent.K2_SetRelativeLocation` _table (`KismetMathLibrary.VLerp` (0.0 0.0 1000.0) (0.0 0.0 -36.0) _fall) false false))
    (:`Finished`
      (bind (_direction_2 _shake) (`Timeline|Shake` :!via `PlayFromStart`)
        (:`Update`
          (`SceneComponent.K2_SetRelativeLocationAndRotation` _table (`KismetMathLibrary.MakeVector` 0.0 0.0 (+ -35.0 (* 5 (`KismetMathLibrary.Abs` _shake)))) (`KismetMathLibrary.MakeRotator` 0.0 (* 10 _shake)) false false))))))

(fn `UserConstructionScript`)